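; BP_Injector is the fire extinguisher part that sprays agent and reports hits on fires in the VR fire training game.
; The construction script picks a default or powder particle template for FoamGenerator based on the extinguisher Type.
; Each particle collision runs a short sphere trace along the particle direction on a custom channel, and any BP_FireInstance hit receives FoamHit with that Type.
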(event OnParticleCollide(FoamGenerator)
  (params (EventName :type Name :default "None") (EmitterTime :type Float%20%28single-precision%29) (ParticleTime :type Integer) (Location :type Vector :default "0, 0, 0") (Velocity :type Vector :default "0, 0, 0") (Direction :type Vector :default "0, 0, 0") (Normal :type Vector :default "0, 0, 0") (BoneName :type Name :default "None") (PhysMat :type Physical%20Material%20Object%20Reference))
  (bind (_outhit _returnvalue) (Collision|SphereTraceByChannel Location (+ Location Direction) 4e+01 "TraceTypeQuery9" false 0 "None"))
  (if _returnvalue
    (bind _asbp_fire_instance (Utilities|Casting|CastToBP_FireInstance (.HitActor (Collision|BreakHitResult _outhit))))
    (Default|FoamHit _asbp_fire_instance (Variables|Default|GetType))))

(fn ConstructionScript
  (Effects|Components|ParticleSystem|SetTemplate (Variables|Default|GetFoamGenerator) (Utilities|Select :Index (Variables|Default|GetType) :NewEnumerator0 "/Game/VRFireTraining/FireExtinguisher/Particles/PS_ExtinguisherDefault.PS_ExtinguisherDefault" :NewEnumerator1 "/Game/VRFireTraining/FireExtinguisher/Particles/PS_ExtinguisherPowder.PS_ExtinguisherPowder" :NewEnumerator2 "/Game/VRFireTraining/FireExtinguisher/Particles/PS_ExtinguisherDefault.PS_ExtinguisherDefault" :NewEnumerator3 "/Game/VRFireTraining/FireExtinguisher/Particles/PS_ExtinguisherPowder.PS_ExtinguisherPowder" :NewEnumerator4 "/Game/VRFireTraining/FireExtinguisher/Particles/PS_ExtinguisherPowder.PS_ExtinguisherPowder")))