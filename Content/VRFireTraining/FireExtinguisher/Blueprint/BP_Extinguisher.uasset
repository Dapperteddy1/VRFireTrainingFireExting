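; A grabbable fire extinguisher for VR training, with a label texture chosen by extinguisher type.
; Grab presses from BP_MotionController step it from pickup through pin pull to two-handed use, with glow materials as hints and hand poses adjusted.
; Equipping spawns a BP_Injector in the other hand, swapping the construction-built spline tube for a cable.
; The trigger runs injector foam and a looping timer that drains charge and turns the gauge needle.
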(event Custom|triggerPress
  (bind _injector (Variables|Default|GetInjector))
  ;[1 1 1] Extinguisher core job
  (if (not (Variables|Default|GettriggerPressed))
    (Variables|Default|SettriggerPressed true)
    (Transformation|AddLocalRotation (Variables|Default|GetHandle) "-20.000000, 0, 0" false false)
    (if (> (Variables|Default|GetchargeLevel) 0.0)
      (Utilities|IsValid _injector
        (:Is%20Valid
          (Components|Activation|Activate (Variables|/Game/VRFireTraining/FireExtinguisher/Blueprint/BP_Injector.BP_Injector_C|GetFoamGenerator _injector) false)
          (Audio|Components|Audio|Play (Variables|/Game/VRFireTraining/FireExtinguisher/Blueprint/BP_Injector.BP_Injector_C|GetSoundFoam _injector) 0.0)
          (bind _returnvalue (Utilities|Time|SetTimerbyEvent (delegate Custom|reduceCharge) 0.2 true))
          (Variables|Default|SetchargeTimer _returnvalue))))))

(event Custom|triggerRelease
  (bind _injector (Variables|Default|GetInjector))
  ;[1 1 1] Extinguisher core job
  (if (Variables|Default|GettriggerPressed)
    (Variables|Default|SettriggerPressed false)
    (Transformation|AddLocalRotation (Variables|Default|GetHandle) "20.000000, 0, 0" false false)
    (Utilities|IsValid _injector
      (:Is%20Valid
        (Components|Activation|Deactivate (Variables|/Game/VRFireTraining/FireExtinguisher/Blueprint/BP_Injector.BP_Injector_C|GetFoamGenerator _injector))
        (Audio|Components|Audio|Stop (Variables|/Game/VRFireTraining/FireExtinguisher/Blueprint/BP_Injector.BP_Injector_C|GetSoundFoam _injector))
        (Utilities|Time|ClearandInvalidateTimerbyHandle (Variables|Default|GetchargeTimer))))))

(event Custom|actionPickup
  (params (Attach%20To :type Scene%20Component%20Object%20Reference))
  ;[1 1 1] Actually pickup extinguisher and attach it to hand
  (Utilities|FlowControl|Sequence
    (:then_0
      (Physics|SetSimulatePhysics (Variables|Default|GetExtinguisherBody) false)
      (Transformation|AttachComponentToComponent (VehicleSound|GetRootComponent) Attach%20To "None" "KeepWorld" "KeepWorld" "KeepWorld" true)
      (Variables|Default|SetattachedTo Attach%20To)
      (Audio|Components|Audio|Play (Variables|Default|GetSoundTake) 0.0)
      (if (Variables|/Script/Engine.SceneComponent|GetbHiddenInGame (Variables|Default|GetPin))
        (Variables|Default|SetState "NewEnumerator1")
        (for _array_element (Variables|Default|GetSplineMesh)
          (Rendering|Material|SetMaterial _array_element 0 "/Game/VRFireTraining/Materials/M_GlowHint.M_GlowHint"))
        (else
          (Variables|Default|SetState "NewEnumerator0")
          (for _array_element_2 (Variables|Default|GetSplineMesh)
            (Rendering|Material|SetMaterial _array_element_2 0 "/Game/VRFireTraining/FireExtinguisher/Materials/M_Tube.M_Tube"))
          (Utilities|Casting|CastToBP_MotionController (Components|GetOwner Attach%20To))
          (Rendering|Material|SetMaterial (Variables|Default|GetPin) 0 "/Game/VRFireTraining/Materials/M_GlowHint.M_GlowHint"))))))

(event Custom|actionPinOut
  ;[1 1 1] Take pin out
  (Audio|Components|Audio|Play (Variables|Default|GetSoundPin) 0.0)
  (Variables|Default|SetState "NewEnumerator1")
  (for _array_element (Variables|Default|GetSplineMesh)
    (Rendering|Material|SetMaterial _array_element 0 "/Game/VRFireTraining/Materials/M_GlowHint.M_GlowHint"))
  (Development|SetHiddeninGame (Variables|Default|GetPin) true false))

(event Custom|actionEquip
  (params (InjectorAttachTo :type Scene%20Component%20Object%20Reference))
  ;[1 1 1] Attach extinguisher to hand in working position and attach injector tube to other hand
  (if (!= InjectorAttachTo (Variables|Default|GetattachedTo))
    (Utilities|IsValid (Variables|Default|GetattachedTo)
      (:Is%20Valid
        (bind _asbp_motion_controller (Utilities|Casting|CastToBP_MotionController (Components|GetOwner InjectorAttachTo))) ; Other hand (holding injector)
        (bind _asbp_motion_controller_2 (Utilities|Casting|CastToBP_MotionController (Components|GetOwner (Variables|Default|GetattachedTo)))) ; Hand holding extinguisher
        (Utilities|FlowControl|Sequence
          (:then_0
            (Rendering|SetVisibility (Variables|Default|GetCable) true false)
            (for _array_element (Variables|Default|GetSplineMesh)
              (Rendering|SetVisibility _array_element false false))
            (Rendering|SetVisibility (Variables|Default|GetTube) false false))
          (:then_1
            (Audio|Components|Audio|Play (Variables|Default|GetSoundPin) 0.0)
            (Variables|Default|SetState "NewEnumerator2")
            (Transformation|DetachFromComponent (VehicleSound|GetRootComponent) "KeepWorld" "KeepWorld" "KeepWorld" true)
            (Transformation|SetActorTransform (Math|Transform|MakeTransform "0, 0, 0"))
            (Transformation|AttachComponentToComponent (Variables|/Game/VRFireTraining/Blueprint/BP_MotionController.BP_MotionController_C|GetExtAttach _asbp_motion_controller_2) "None" "KeepRelative" "KeepRelative" "KeepRelative" true)
            (bind _returnvalue (Game|SpawnActorfromClass "/Game/VRFireTraining/FireExtinguisher/Blueprint/BP_Injector.BP_Injector_C" (Math|Transform|MakeTransform "0, 0, 0" "0,180.000000, 0" "0.500000,0.500000,0.500000") "AlwaysSpawn" 0 (Variables|Default|GetType) 0))
            (Transformation|AttachComponentToComponent _returnvalue (Variables|/Game/VRFireTraining/Blueprint/BP_MotionController.BP_MotionController_C|GetExtInjAttach _asbp_motion_controller) "None" "KeepRelative" "KeepRelative" "KeepRelative" true)
            (Class|CableComponent|SetAttachEndtoComponent (Variables|Default|GetCable) (Variables|Default|GetCableEnd) "None")
            (Variables|Default|SetInjector _returnvalue)
            (Transformation|AttachComponentToComponent (Variables|Default|GetCableEnd) (Variables|/Game/VRFireTraining/FireExtinguisher/Blueprint/BP_Injector.BP_Injector_C|Getend _returnvalue) "None" "SnapToTarget" "SnapToTarget" "KeepWorld" true))
          (:then_2
            (Utilities|FlowControl|Sequence
              (:then_0
                (bind _asbpa_hand (Utilities|Casting|CastToBPA_Hand (Components|SkeletalMesh|GetAnimInstance (Variables|/Game/VRFireTraining/Blueprint/BP_MotionController.BP_MotionController_C|GetHandMesh _asbp_motion_controller_2))))
                (Variables|/Game/VRFireTraining/Hands/Animations/BPA_Hand.BPA_Hand_C|Setgripcf _asbpa_hand 2e+01)
                (Variables|/Game/VRFireTraining/Hands/Animations/BPA_Hand.BPA_Hand_C|Setgripadd _asbpa_hand 0.7))
              (:then_1
                (bind _asbpa_hand_2 (Utilities|Casting|CastToBPA_Hand (Components|SkeletalMesh|GetAnimInstance (Variables|/Game/VRFireTraining/Blueprint/BP_MotionController.BP_MotionController_C|GetHandMesh _asbp_motion_controller))))
                (Variables|/Game/VRFireTraining/Hands/Animations/BPA_Hand.BPA_Hand_C|Setgripcf _asbpa_hand_2 1e+02)
                (Variables|/Game/VRFireTraining/Hands/Animations/BPA_Hand.BPA_Hand_C|Setgripadd _asbpa_hand_2 0.8))
              (:then_2
                (Transformation|AddLocalRotation (Variables|/Game/VRFireTraining/Blueprint/BP_MotionController.BP_MotionController_C|GetHandMesh _asbp_motion_controller_2) (Math|Rotator|MakeRotator 0.0 0.0 4e+01) false false)
                (Default|EquipEstinguisher _asbp_motion_controller_2 self))
              (:then_3
                (Transformation|AddLocalRotation (Variables|/Game/VRFireTraining/Blueprint/BP_MotionController.BP_MotionController_C|GetHandMesh _asbp_motion_controller) (Math|Rotator|MakeRotator 0.0 0.0 85.0) false false))))
          (:then_3
            (Variables|Default|SetInjectorAttachedTo InjectorAttachTo)))))))

(event Custom|actionUnequip
  (bind _attachedto (Variables|Default|GetattachedTo))
  (bind _injectorattachedto (Variables|Default|GetInjectorAttachedTo))
  ;[1 1 1] Attach extinguisher to hand in working position and attach injector tube to other hand
  (Utilities|FlowControl|Sequence
    (:then_0
      (Utilities|IsValid _attachedto
        (:Is%20Valid
          (bind _asbp_motion_controller (Utilities|Casting|CastToBP_MotionController (Components|GetOwner _attachedto)))
          (Transformation|AddLocalRotation (Variables|/Game/VRFireTraining/Blueprint/BP_MotionController.BP_MotionController_C|GetHandMesh _asbp_motion_controller) (Math|Rotator|MakeRotator 0.0 0.0 -4e+01) false false)
          (bind _asbpa_hand (Utilities|Casting|CastToBPA_Hand (Components|SkeletalMesh|GetAnimInstance (Variables|/Game/VRFireTraining/Blueprint/BP_MotionController.BP_MotionController_C|GetHandMesh _asbp_motion_controller))))
          (Variables|/Game/VRFireTraining/Hands/Animations/BPA_Hand.BPA_Hand_C|Setgripcf _asbpa_hand 2.0)
          (Variables|/Game/VRFireTraining/Hands/Animations/BPA_Hand.BPA_Hand_C|Setgripadd _asbpa_hand 0.0))))
    (:then_1
      (Utilities|IsValid _injectorattachedto
        (:Is%20Valid
          (bind _asbp_motion_controller_2 (Utilities|Casting|CastToBP_MotionController (Components|GetOwner _injectorattachedto)))
          (Transformation|AddLocalRotation (Variables|/Game/VRFireTraining/Blueprint/BP_MotionController.BP_MotionController_C|GetHandMesh _asbp_motion_controller_2) (Math|Rotator|MakeRotator 0.0 0.0 -85.0) false false)
          (bind _asbpa_hand_2 (Utilities|Casting|CastToBPA_Hand (Components|SkeletalMesh|GetAnimInstance (Variables|/Game/VRFireTraining/Blueprint/BP_MotionController.BP_MotionController_C|GetHandMesh _asbp_motion_controller_2))))
          (Variables|/Game/VRFireTraining/Hands/Animations/BPA_Hand.BPA_Hand_C|Setgripcf _asbpa_hand_2 2.0)
          (Variables|/Game/VRFireTraining/Hands/Animations/BPA_Hand.BPA_Hand_C|Setgripadd _asbpa_hand_2 0.0))))
    (:then_2
      (Transformation|DetachFromComponent (Variables|Default|GetCableEnd) "KeepWorld" "KeepWorld" "KeepWorld" true))
    (:then_3
      (CallFunction|TriggerRelease)
      (bind _asbp_motion_controller_3 (Utilities|Casting|CastToBP_MotionController (Components|GetOwner (Variables|Default|GetattachedTo)))) ; Other hand (holding injector)
      (Default|ReleaseExtinguisher _asbp_motion_controller_3)
      (Actor|DestroyActor (Variables|Default|GetInjector))
      (Rendering|SetVisibility (Variables|Default|GetCable) false false)
      (for _array_element (Variables|Default|GetSplineMesh)
        (Rendering|SetVisibility _array_element true false))
      (Rendering|SetVisibility (Variables|Default|GetTube) true false))))

(event Custom|reduceCharge
  (bind _injector (Variables|Default|GetInjector))
  ;[1 1 1] Extinguisher core job
  (bind _output_get (Variables|Default|SetchargeLevel (Math|Float|Max(Float) (- (Variables|Default|GetchargeLevel) 0.2) 0.0)))
  (CallFunction|UpdateChargeIndicator)
  (if (== _output_get 0.0)
    (Utilities|IsValid _injector
      (:Is%20Valid
        (Components|Activation|Deactivate (Variables|/Game/VRFireTraining/FireExtinguisher/Blueprint/BP_Injector.BP_Injector_C|GetFoamGenerator _injector))
        (Audio|Components|Audio|Stop (Variables|/Game/VRFireTraining/FireExtinguisher/Blueprint/BP_Injector.BP_Injector_C|GetSoundFoam _injector))
        (Utilities|Time|ClearandInvalidateTimerbyHandle (Variables|Default|GetchargeTimer))))))

(event Custom|updateChargeIndicator
  ;[1 1 1] Extinguisher core job
  (Transformation|SetRelativeRotation (Variables|Default|GetchargeIndicator) (Math|Rotator|MakeRotator 0.0 (* (- 1.0 (Math|Float|Clamp(Float) (/ (Variables|Default|GetchargeLevel) (Variables|Default|GetinitialCharge)))) 65.0) 0.0) false false))

(event EventBeginPlay
  ;[1 1 1] begin Play
  (Physics|SetSimulatePhysics (Variables|Default|GetExtinguisherBody) true)
  (Rendering|SetVisibility (Variables|Default|GetCable) false false)
  (Variables|Default|SetinitialCharge (Variables|Default|GetchargeLevel))
  (CallFunction|UpdateChargeIndicator))

(event EventPickup
  (params (AttachTo :type Scene%20Component%20Object%20Reference))
  ;[1 1 1] Pickup interface (actions done on grab button)
  (Utilities|Casting|CastToBP_MotionController (Components|GetOwner AttachTo))
  (switch Utilities|FlowControl|Switch|SwitchonENUM_ExtinguisherState (Variables|Default|GetState)
    (:NewEnumerator3
      (CallFunction|ActionPickup AttachTo))
    (:NewEnumerator0
      (if (> (Utilities|Array|Length (Class|PrimitiveComponent|GetOverlappingComponents (Variables|Default|GetRingCollision))) 0)
        (CallFunction|ActionPinOut)))
    (:NewEnumerator1
      (if (> (Utilities|Array|Length (Class|PrimitiveComponent|GetOverlappingComponents (Variables|Default|GetInjCollision))) 0)
        (CallFunction|ActionEquip AttachTo)))))

(event EventDrop
  ;[1 1 1] Pickup interface (actions done on grab button)
  (Transformation|DetachFromComponent (VehicleSound|GetRootComponent) "KeepWorld" "KeepWorld" "KeepWorld" true)
  (Utilities|FlowControl|Sequence
    (:then_0
      (switch Utilities|FlowControl|Switch|SwitchonENUM_ExtinguisherState (Variables|Default|GetState)
        (:NewEnumerator2
          (CallFunction|ActionUnequip))))
    (:then_1
      (Physics|SetSimulatePhysics (Variables|Default|GetExtinguisherBody) true)
      (Class|PrimitiveComponent|SetAllPhysicsLinearVelocity (Variables|Default|GetExtinguisherBody) "0, 0, 0" false)
      (Variables|Default|SetattachedTo 0)
      (Variables|Default|SetState "NewEnumerator3")
      (Rendering|Material|SetMaterial (Variables|Default|GetPin) 0 "/Game/VRFireTraining/FireExtinguisher/Materials/M_Gold.M_Gold")
      (for _array_element (Variables|Default|GetSplineMesh)
        (Rendering|Material|SetMaterial _array_element 0 "/Game/VRFireTraining/FireExtinguisher/Materials/M_Tube.M_Tube")))))

(fn ConstructionScript
  (bind _spline (Variables|Default|GetSpline))
  (bind _spline_2 (Variables|Default|GetSpline))
  (bind _extinguisherbody (Variables|Default|GetExtinguisherBody))
  ;[1 1 1] Generate spline mesh (tube)
  (Utilities|FlowControl|Sequence
    (:then_0
      (for _index (range 0 (- (Spline|GetNumberOfSplinePoints _spline) 1))
        (bind _returnvalue (AddComponent|AddSplineMeshComponent false (Transformation|GetRelativeTransform _spline)))
        (SplineMesh|SetForwardAxis _returnvalue "Z" true)
        (SplineMesh|SetStartandEnd _returnvalue (Spline|GetLocationatSplinePoint _spline_2 _index "Local") (Spline|GetTangentatSplinePoint _spline_2 _index "Local") (Spline|GetLocationatSplinePoint _spline_2 (+ _index 1) "Local") (Spline|GetTangentatSplinePoint _spline_2 (+ _index 1) "Local") true :!class /Script/Engine.SplineMeshComponent)
        (Utilities|Array|Add (Variables|Default|GetSplineMesh) _returnvalue)
        (Transformation|AttachComponentToComponent _returnvalue (Variables|Default|GetExtinguisherBody) "None" "KeepRelative" "KeepRelative" "KeepRelative" true)))
    (:then_1
      (bind _returnvalue_2 (Rendering|Material|CreateDynamicMaterialInstance _extinguisherbody 0 0 "None" :!class /Script/Engine.PrimitiveComponent))
      (Rendering|Material|SetMaterial _extinguisherbody 0 _returnvalue_2)
      (Rendering|Material|SetTextureParameterValue _returnvalue_2 "TextureParam" (Utilities|Select :Index (Variables|Default|GetType) :NewEnumerator0 "/Game/VRFireTraining/FireExtinguisher/TextureExtinguisher/T_ExtinguisherWater.T_ExtinguisherWater" :NewEnumerator1 "/Game/VRFireTraining/FireExtinguisher/TextureExtinguisher/T_ExtinguisherCO2.T_ExtinguisherCO2" :NewEnumerator2 "/Game/VRFireTraining/FireExtinguisher/TextureExtinguisher/T_ExtinguisherFoam.T_ExtinguisherFoam" :NewEnumerator3 "/Game/VRFireTraining/FireExtinguisher/TextureExtinguisher/T_ExtinguisherPowder.T_ExtinguisherPowder" :NewEnumerator4 "/Game/VRFireTraining/FireExtinguisher/TextureExtinguisher/T_ExtinguisherWet.T_ExtinguisherWet")))))