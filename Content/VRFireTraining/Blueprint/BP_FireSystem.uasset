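; Fire spread manager for VR fire training that starts a fire at a set point and grows it until all fires are out.
; On Tick, at a rate set by ExpandRate and up to MaxFires, it tries random nearby points around shuffled existing BP_FireInstances.
; Sphere traces reject spots near active fires, find flammable surfaces and pick each fire's type by trace channel.
; When an expiring instance leaves none active, it announces success.
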(event Custom|startFire
  ;[1 1 1] Start Event - you can call this from your blueprints to start the fire
  (Variables|Default|SetisActive true)
  (CallFunction|ExpandFire (Transformation|GetWorldLocation (Variables|Default|GetFireStartPosition))))

(event Custom|stopAll
  (bind _instances (Variables|Default|GetInstances))
  ;[1 1 1] stops all the fires and destroys them (usefull to reset level)
  (for _array_element _instances
    (Actor|DestroyActor _array_element)
    (Utilities|Array|RemoveItem _instances _array_element)))

(event Custom|onFireInstanceExpired
  (bind _numactive (CallFunction|CountActiveFires))
  (if (== _numactive 0)
    (CallFunction|OnAllFiresStopped)))

(event Custom|onAllFiresStopped
  ;[1 1 1] This event is called when you have stopped all fires
  (Development|PrintString "You have stopped all the fire!"))

(event EventBeginPlay
  (if (Variables|Default|GetActivate)
    (CallFunction|StartFire)))

(event EventTick
  (params (DeltaSeconds :type Float%20%28single-precision%29))
  (if (Variables|Default|GetisActive)
    ;[1 1 1] Check if we can spawn a new fire, depending on time and expandRate
    (if (> (Utilities|Time|GetGameTimeinSeconds) (+ (Variables|Default|GetlastSpawnedTS) (/ 3e+02 (Variables|Default|GetexpandRate))))
      ;[1 1 1] skip spawn if we have no fires or reached maximum fires
      (bind _numactive (CallFunction|CountActiveFires))
      (if (not (== _numactive 0))
        (if (< _numactive (Variables|Default|GetmaxFires))
          ;[1 1 1] Spawn near some of existing fires (randomly selected)
          (bind _array_element (Utilities|Array|ForEachLoopwithBreak (Variables|Default|GetInstances) :!label _label)
            (:LoopBody
              (bind _spawned (CallFunction|ExpandFire (Transformation|GetActorLocation _array_element)))
              (if _spawned
                (Utilities|Array|Shuffle (Variables|Default|GetInstances))
                (goto _label Break))))
          (else
            (Variables|Default|SetlastSpawnedTS (Utilities|Time|GetGameTimeinSeconds))))))))

(fn ConstructionScript
  (bind _mindistance (Variables|Default|GetminDistance))
  (bind _returnvalue (+ _mindistance 1e+01))
  (if (< (Variables|Default|GetsearchRadius) _returnvalue)
    (Variables|Default|SetsearchRadius _returnvalue)))

(fn ExpandFire
  (params (location :type Vector))
  (bind _returnvalue (Math|Random|RandomFloatinRange -9999.0 9999.0))
  (bind _searchradius (Variables|Default|GetsearchRadius))
  (bind _returnvalue_2 (Math|Vector|MakeVector _searchradius 0.0 0.0))
  (bind _returnvalue_3 (Math|Vector|RotateVectorAroundAxis _returnvalue_2 _returnvalue "0.000000, 0,1.000000"))
  (bind (_spawned _instance) (CallFunction|TrySpawn location location))
  (if _spawned
    (return _instance true)
    (else
      (bind (_spawned_2 _instance_2) (CallFunction|TrySpawn location (+ location _returnvalue_3)))
      (if _spawned_2
        (return _instance_2 true)
        (else
          (bind (_spawned_3 _instance_3) (CallFunction|TrySpawn location (+ location (Math|Vector|RotateVectorAroundAxis _returnvalue_3 9e+01 "0.000000, 0,1.000000"))))
          (if _spawned_3
            (return _instance_3 true)
            (else
              (bind (_spawned_4 _instance_4) (CallFunction|TrySpawn location (+ location (Math|Vector|RotateVectorAroundAxis _returnvalue_3 1.8e+02 "0.000000, 0,1.000000"))))
              (if _spawned_4
                (return _instance_4 true)
                (else
                  (bind (_spawned_5 _instance_5) (CallFunction|TrySpawn location (+ location (Math|Vector|RotateVectorAroundAxis _returnvalue_3 1.8e+02 "0.000000, 0,1.000000"))))
                  (return _instance_5 _spawned_5))))))))))

(fn TrySpawn
  (params (location :type Vector) (newLocation :type Vector))
  (bind _returnvalue (+ newLocation "0, 0,1.000000"))
  ;[1 1 1] Check that we don't have existing fire nearby
  (bind (_outhit _returnvalue_2) (Collision|SphereTraceByChannel newLocation _returnvalue (Variables|Default|GetminDistance) "TraceTypeQuery9" false 0 "None" true "(R=0.000000,G=0.361571,B=1.000000,A=1.000000)" "(R=0.994898,G=1.000000,B=0.000000,A=1.000000)" 3.0))
  (if _returnvalue_2
    ;[1 1 1] If its unactive we can still spawn here
    (bind _asbp_fire_instance (Utilities|Casting|CastToBP_FireInstance (.HitActor (Collision|BreakHitResult _outhit)))
      (:then
        (if (Variables|/Game/VRFireTraining/Blueprint/BP_FireInstance.BP_FireInstance_C|GetisActive _asbp_fire_instance)
          (return false 0)
          (elif (Variables|Default|GetcanSpawnOnExpired)
            _
            (else
              (return false 0)))))
      (:CastFailed
        _)))
  ;[1 1 1] Find any flameable objects in the area
  (bind (_outhit_2 _returnvalue_3) (Collision|SphereTraceByChannel newLocation _returnvalue (Variables|Default|GetsearchRadius) "TraceTypeQuery3" false 0 "None"))
  (if _returnvalue_3
    ;[1 1 1] Detect type of the area and spawn fire instance
    (bind _type (CallFunction|FindType (.ImpactPoint (Collision|BreakHitResult _outhit_2))))
    (bind _returnvalue_4 (Game|SpawnActorfromClass "/Game/VRFireTraining/Blueprint/BP_FireInstance.BP_FireInstance_C" (Math|Transform|MakeTransform (.ImpactPoint (Collision|BreakHitResult _outhit_2))) "AlwaysSpawn" 0 _type self (Variables|Default|GetexpireTime) (Variables|Default|GetfireStrength) (Variables|Default|GetQuality) 0))
    (Utilities|Array|Add (Variables|Default|GetInstances) _returnvalue_4)
    (Variables|Default|SetlastSpawnedTS (Utilities|Time|GetGameTimeinSeconds))
    (return true _returnvalue_4)
    (else
      (return false 0))))

(fn FindType
  (params (location :type Vector))
  (bind _returnvalue (+ location "0, 0,10.000000"))
  (bind _returnvalue_2 (Collision|SphereTraceByChannel location _returnvalue 5.0 "TraceTypeQuery4" false 0 "None"))
  (if _returnvalue_2
    (return "NewEnumerator0")
    (else
      (bind _returnvalue_3 (Collision|SphereTraceByChannel location _returnvalue 5.0 "TraceTypeQuery5" false 0 "None"))
      (if _returnvalue_3
        (return "NewEnumerator1")
        (else
          (bind _returnvalue_4 (Collision|SphereTraceByChannel location _returnvalue 5.0 "TraceTypeQuery6" false 0 "None"))
          (if _returnvalue_4
            (return "NewEnumerator2")
            (else
              (bind _returnvalue_5 (Collision|SphereTraceByChannel location _returnvalue 5.0 "TraceTypeQuery7" false 0 "None"))
              (if _returnvalue_5
                (return "NewEnumerator3")
                (else
                  (bind _returnvalue_6 (Collision|SphereTraceByChannel location _returnvalue 5.0 "TraceTypeQuery8" false 0 "None"))
                  (if _returnvalue_6
                    (return "NewEnumerator4")
                    (else
                      (return "NewEnumerator5"))))))))))))

(fn CountActiveFires
  (for _array_element (Variables|Default|GetInstances)
    (if (Variables|/Game/VRFireTraining/Blueprint/BP_FireInstance.BP_FireInstance_C|GetisActive _array_element)
      (Math|Integer|IncrementInt (LocalVariables|Getcnt))))
  (return (LocalVariables|Getcnt)))