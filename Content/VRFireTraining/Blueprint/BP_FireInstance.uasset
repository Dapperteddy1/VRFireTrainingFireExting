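; A single fire in the VR fire training game, with a fire type, health and a timed lifetime.
; Quality picks a sprite or volumetric particle effect, and high-quality wood, liquid and metal fires also show a mesh that scales up via timeline.
; FoamHit damages the fire only when the extinguisher type suits the fire type.
; At zero health or timeout, it disables visuals and collision and notifies its owning fire system.
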(event Custom|expire
  ;[1 1 1] expire Event (stop current fire)
  (Utilities|Time|ClearandInvalidateTimerbyHandle (Variables|Default|GetexpireTimer))
  (Components|Activation|Deactivate (Variables|Default|GetParticleSystem))
  (Variables|Default|SetisActive false)
  (Collision|SetCollisionEnabled (Variables|Default|GetSphere) "NoCollision")
  (Rendering|SetVisibility (Variables|Default|GetFireMesh) false true)
  (Default|OnFireInstanceExpired (Variables|Default|GetmySystem)))

(event Custom|FoamHit
  (params (Type :type ENUM_ExtinguisherType%20Enum :default "NewEnumerator0"))
  ;[1 1 1] Extinguisher interaction based on fire type and extinguisher type
  (switch Utilities|FlowControl|Switch|SwitchonENUM_FireType (Variables|Default|GetType)
    (:NewEnumerator0
      (if (Utilities|Select :Index Type :NewEnumerator0 true :NewEnumerator1 false :NewEnumerator2 true :NewEnumerator3 true :NewEnumerator4 true)
        (bind _output_get (Variables|Default|Sethealth (Math|Float|Max(Float) (- (Variables|Default|Gethealth) 3e+01) 0.0) :!label _label))
        (if (<= _output_get 0.0)
          (CallFunction|Expire))))
    (:NewEnumerator1
      (if (Utilities|Select :Index Type :NewEnumerator0 false :NewEnumerator1 true :NewEnumerator2 true :NewEnumerator3 true :NewEnumerator4 true)
        (goto _label)))
    (:NewEnumerator2
      (if (Utilities|Select :Index Type :NewEnumerator0 false :NewEnumerator1 true :NewEnumerator2 false :NewEnumerator3 true :NewEnumerator4 false)
        (goto _label)))
    (:NewEnumerator3
      (if (Utilities|Select :Index Type :NewEnumerator0 false :NewEnumerator1 false :NewEnumerator2 false :NewEnumerator3 true :NewEnumerator4 false)
        (goto _label)))
    (:NewEnumerator4
      (if (Utilities|Select :Index Type :NewEnumerator0 false :NewEnumerator1 false :NewEnumerator2 false :NewEnumerator3 true :NewEnumerator4 false)
        (goto _label)))))

(event EventBeginPlay
  (bind _returnvalue (Utilities|Time|SetTimerbyEvent (delegate Custom|expire) (Variables|Default|GetexpireTime)))
  (Variables|Default|SetexpireTimer _returnvalue)
  (switch Utilities|FlowControl|Switch|SwitchonENUM_Quality (Variables|Default|GetQuality)
    (:NewEnumerator0
      (Rendering|SetVisibility (Variables|Default|GetFireMesh) false true :!label _label)
      (Components|Activation|Activate (Variables|Default|GetParticleSystem) false))
    (:NewEnumerator1
      (switch Utilities|FlowControl|Switch|SwitchonENUM_FireType (Variables|Default|GetType)
        (:NewEnumerator0
          _)
        (:NewEnumerator1
          _)
        (:NewEnumerator2
          (goto _label))
        (:NewEnumerator3
          _)
        (:NewEnumerator4
          (goto _label)))
      (Rendering|SetVisibility (Variables|Default|GetFireMesh) true true)
      (bind _scale (Timeline|Timeline_0 PlayFromStart)
        (:Update
          (Transformation|SetRelativeScale3D (Variables|Default|GetFireMesh) (Math|Vector|MakeVector _scale _scale _scale)))))))

(fn ConstructionScript
  (bind _particlesystem (Variables|Default|GetParticleSystem))
  (Effects|Components|ParticleSystem|SetTemplate _particlesystem (Utilities|Select :Index (Variables|Default|GetQuality) :NewEnumerator0 "/Game/VRFireTraining/FireVFX/Particles/PS_SpriteFlame.PS_SpriteFlame" :NewEnumerator1 "/Game/VRFireTraining/FireVFX/Particles/PS_VolumeFire.PS_VolumeFire"))
  (Transformation|SetRelativeRotation _particlesystem (Utilities|Select :Index (Variables|Default|GetQuality) :NewEnumerator0 "0, 0, 0" :NewEnumerator1 "-90.000000,0.000000, 0") false false))